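; BP_Clock is an actor that shows the current time of day and disappears when the third-person character hits it.
; Each Tick bobs it vertically around its BeginPlay location with a sine of game time and writes the system time to its TextRender.
; A Cylinder hit by BP_ThirdPersonCharacter plays a click sound at its location and destroys the actor.
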(event `self.ReceiveBeginPlay`
  (set `self.Origin` (`self.K2_GetActorLocation`)))

(event `self.ReceiveTick`
  (params (DeltaSeconds :type "Float (single-precision)"))
  (`self.K2_SetActorLocation` (`KismetMathLibrary.MakeVector` (.x (`self.Origin`)) (.y (`self.Origin`)) (+ (.z (`self.Origin`)) (* (`KismetMathLibrary.Sin` (`GameplayStatics.GetTimeSeconds`)) 50.0))))
  (`TextRenderComponent.K2_SetText` (`self.TextRender`) (`KismetTextLibrary.AsTimespan_Timespan` (`KismetMathLibrary.GetTimeOfDay` (`KismetMathLibrary.Now`)))))

(event `self.Cylinder.OnComponentHit`
  (params (HitComponent :type "PrimitiveComponent Object Reference") (OtherActor :type "Actor Object Reference") (OtherComp :type "PrimitiveComponent Object Reference") (NormalImpulse :type "Vector Structure") (Hit :type "HitResult Structure (by ref)"))
  (cast `/Game/ThirdPerson/Blueprints/BP_ThirdPersonCharacter` OtherActor)
  (`GameplayStatics.PlaySoundAtLocation` "/Engine/VREditor/Sounds/VR_click1.VR_click1" (`self.K2_GetActorLocation`) (struct) 1.0 1.0 0.0 null null null null)
  (`self.K2_DestroyActor`))

(fn `UserConstructionScript`)